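; BP_KeyBearer is a one-time interactable from which the player picks up a key.
; It supplies its root transform and a pickup montage for the player's interaction animation.
; Interacting sets KeyPickedUp to block reuse, plays the corpse and key animations, then destroys the key component after its animation length.
; It then sends a KeyPickedUp StateTree event to the first BP_EnemyController found, signalling the enemy AI.
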(event Custom|StartPickup
  (bind _a_takekey (Variables|Default|GetA_TakeKey))
  (Variables|Default|SetbKeyPickedUp true)
  (Audio|Components|Audio|Play (Variables|Default|GetA_Corpse) false)
  (Audio|Components|Audio|Play _a_takekey false)
  (Utilities|FlowControl|Delay (Animation|GetPlayLength (.AnimToPlay (Utilities|Struct|BreakSingleAnimationPlayData (Variables|/Script/Engine.SkeletalMeshComponent|GetAnimationData _a_takekey)))))
  (Components|DestroyComponent (Variables|Default|GetA_TakeKey))
  (bind _returnvalue (Actor|GetActorOfClass "/Game/InteractionTestTask/Enemy/BP_EnemyController.BP_EnemyController_C"))
  (Gameplay|StateTree|SendStateTreeEvent (Variables|/Game/InteractionTestTask/Enemy/BP_EnemyController.BP_EnemyController_C|GetStateTreeAI _returnvalue) (Utilities|Struct|MakeStateTreeEvent "(TagName=\"Test.StateTree.KeyPickedUp\")" "KeyBearer") :!class /Script/GameplayStateTreeModule.StateTreeComponent))

(event EventInteract
  (CallFunction|StartPickup))

(fn ConstructionScript)

(fn GetCanInteract
  (return (not (Variables|Default|GetbKeyPickedUp))))

(fn GetInteractAnimationData
  (return (Transformation|GetWorldTransform (Variables|Default|GetRoot)) (Variables|Default|GetPickupKeyMontage)))