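; Enemy AI controller that runs a StateTree for its behavior and tracks whether it can see the player.
; On BeginPlay it starts the StateTree logic.
; AI Perception updates are filtered to sight stimuli from the player pawn, setting PlayerPawn when seen and clearing it when sight is lost.
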(event OnTargetPerceptionUpdated(AIPerception)
  (params (Actor :type Actor%20Object%20Reference) (Stimulus :type AI%20Stimulus%20Structure))
  (CallFunction|TryProcessSightSense Actor Stimulus))

(event EventBeginPlay
  (AI|Logic|StartLogic (Variables|Default|GetStateTreeAI)))

(event EventTick
  (params (DeltaSeconds :type Float%20%28single-precision%29)))

(fn ConstructionScript)

(fn TryProcessSightSense
  (params (SeenActor :type Actor%20Object%20Reference) (Stimulus :type AI%20Stimulus%20Structure))
  (bind _returnvalue (Class|AIPerceptionSystem|GetSenseClassforStimulus Stimulus))
  (if (== _returnvalue "/Script/AIModule.AISense_Sight")
    (if (== SeenActor (Game|Player|GetPlayerPawn 0))
      (if (.bsuccessfullysensed Stimulus)
        ;[1 1 1] Seen the player
        (bind _aspawn (Utilities|Casting|CastToPawn SeenActor))
        (Variables|Default|SetPlayerPawn _aspawn)
        (else
          ;[1 1 1] Lost the player
          (Variables|Default|SetPlayerPawn 0)))
      (else
        ;[1 0 0.02604] Seen, but not the player
        (return)))
    (else
      ;[1 0.06418 0] Not sight stimulus
      (return))))