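; BP_LookInteractorComponent is a scene component that lets its owner interact with whatever actor it faces.
; TryInteract runs a debug-drawn Visibility line trace along the component's forward vector, up to a maximum distance.
; Through interface messages, it checks whether the hit actor can be interacted with, triggers the interaction and fetches its animation data.
; It then broadcasts a successful-interaction event carrying the target player origin and montage.
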(event EventBeginPlay)

(event EventTick
  (params (DeltaSeconds :type Float%20%28single-precision%29)))

(fn TryInteract
  (bind _returnvalue (Transformation|GetWorldLocation))
  (bind (_outhit _returnvalue_2) (Collision|LineTraceByChannel _returnvalue (+ _returnvalue (* (Math|Vector|GetForwardVector) (Variables|Default|GetMaxInteractionDistance))) "TraceTypeQuery1" false 0 "ForDuration"))
  (if _returnvalue_2
    (bind _bcaninteract (Class|BPIInteractableActor|GetCanInteract(Message) (.HitActor (Collision|BreakHitResult _outhit))))
    (if _bcaninteract
      (Class|BPIInteractableActor|Interact(Message) (.HitActor (Collision|BreakHitResult _outhit)))
      (bind (_targetplayerorigin _interactionmontage) (Class|BPIInteractableActor|GetInteractAnimationData(Message) (.HitActor (Collision|BreakHitResult _outhit))))
      (Default|CallOnSuccessfulInteraction _targetplayerorigin _interactionmontage))))