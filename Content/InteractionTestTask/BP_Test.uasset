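; BP_Test is a test character Blueprint for a key pickup interaction, driven by a RunTest event.
; RunTest finds the BP_KeyBearer, starts its pickup and reads the player target transform from it.
; It then enables orient-to-movement, plays the take-key montage and sets the actor directly to that transform.
; A Motion Warping target update for the pickup position exists but is disconnected, so it never runs.
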(event Custom|RunTest
  (bind _returnvalue (Actor|GetActorOfClass "/Game/InteractionTestTask/BP_KeyBearer.BP_KeyBearer_C"))
  (Default|StartPickup _returnvalue)
  (bind _targettransform (Default|GetPlayerTargetTransform _returnvalue))
  (Variables|/Script/Engine.CharacterMovementComponent|SetbOrientRotationToMovement (Variables|Character|GetCharacterMovement) true)
  (Animation|PlayAnimMontage "/Game/InteractionTestTask/SourceAssets/Character/AM_Character_TakeKey.AM_Character_TakeKey" 1.0 "None")
  (Transformation|SetActorTransform (Math|Transform|MakeTransform (+ (.Location (Math|Transform|BreakTransform _targettransform)) "0.000000,0.000000,0.000000") (.Rotation (Math|Transform|BreakTransform _targettransform)) "1.000000,1.000000,1.000000")))

(event EventBeginPlay)

(event Collision|EventActorBeginOverlap
  (params (OtherActor :type Actor%20Object%20Reference)))

(event EventTick
  (params (DeltaSeconds :type Float%20%28single-precision%29)))

(fn ConstructionScript)